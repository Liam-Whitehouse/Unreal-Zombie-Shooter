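; Gameplay ability for player death that plays a death montage and sinks the avatar downward.
; On activation it commits, starts the montage, then loops each tick through a zero-length RetriggerableDelay.
; Each pass interpolates toward 100 units below the current location without sweep, giving a steady descent rather than a fixed end point.
; The graph never ends the ability; its comment says code in HandleRespawn cancels or ends it.
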(event Ability|EventActivateAbility
  (bind _returnvalue (Ability|GetAvatarActorfromActorInfo))
  (bind _returnvalue_2 (Transformation|GetActorLocation _returnvalue))
  ;[1 1 1] This ability gets cancelled/ended in Code inside of HandleRespawn
  (Ability|CommitAbility)
  (|PlayMontageandWaitProxy "None" "/Game/Stylized_Death/Meshes/Animation/AM_Deathy_Death_B.AM_Deathy_Death_B" 1.0 "None" true 1.0 0.0 false
    (:then
      (Transformation|SetActorLocation (Ability|GetAvatarActorfromActorInfo) (Math|Interpolation|VInterpTo (Transformation|GetActorLocation (Ability|GetAvatarActorfromActorInfo)) (Math|Vector|MakeVector (.x _returnvalue_2) (.y _returnvalue_2) (- (.z _returnvalue_2) 1e+02)) (Utilities|Time|GetWorldDeltaSeconds) 1.0) false false :!label _label)
      (Utilities|FlowControl|RetriggerableDelay 0.0)
      (goto _label))))