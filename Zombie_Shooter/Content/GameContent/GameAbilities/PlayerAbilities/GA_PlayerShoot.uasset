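; GA_PlayerShoot is a player gameplay ability that fires a hitscan shot.
; On activation it commits, rolls the CriticalChance attribute to add a critical tag, and plays a fast-shoot montage, ending when that finishes.
; With authority, it line-traces from the camera with debug drawing, applies the damage effect to a hit Pawn, then clears the critical tag.
; A miss leaves the tag in place, and the computed muzzle vector is unused by the trace.
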(event Ability|EventActivateAbility
  (bind _returnvalue (Ability|GetAvatarActorfromActorInfo))
  (bind _returnvalue_2 (Ability|GetAvatarActorfromActorInfo))
  (bind _returnvalue_3 (Actor|GetComponentbyClass _returnvalue "/Script/Engine.SkeletalMeshComponent"))
  (bind _returnvalue_4 (Actor|GetComponentbyClass _returnvalue_2 "/Script/Engine.CameraComponent"))
  (bind _returnvalue_5 (Transformation|GetWorldLocation _returnvalue_4))
  (Ability|CommitAbility)
  (Variables|Default|SetOwningASC (.AsZombie%20Ability%20System%20Component (Utilities|Casting|CastToZombieAbilitySystemComponent (Ability|GetAbilitySystemComponent (Ability|GetAvatarActorfromActorInfo)))))
  (if (<= (Math|Random|RandomIntegerinRange 0 100) (.CurrentValue (Utilities|Struct|BreakGameplayAttributeData (Variables|/Script/Zombie_Shooter.ZombieAttributeSet|GetCriticalChance (.AsZombie%20Attribute%20Set (Utilities|Casting|CastToZombieAttributeSet (Class|BaseCharacter|GetAttributeSet (.AsBase%20Character (Utilities|Casting|CastToBaseCharacter (Ability|GetAvatarActorfromActorInfo))))))))))
    (Class|ZombieAbilitySystemComponent|AddGameplayTag (Variables|Default|GetOwningASC) (Variables|Default|GetCriticalTag)))
  (|PlayMontageandWaitProxy "None" "/Game/GameContent/Player/Animations/AM_Deathy_FastShoot.AM_Deathy_FastShoot" 1.0 "None" true 1.0 0.0 true
    (:then
      (Ability|HasAuthority
        (:True
          (Variables|Default|SetGunMuzzleVector (+ (Transformation|GetSocketLocation _returnvalue_3 "Muzzle_01") (Math|Vector|GetForwardVector (Transformation|GetSocketRotation _returnvalue_3 "Muzzle_01"))))
          (bind _outhit (Collision|LineTraceByChannel _returnvalue_5 (+ _returnvalue_5 (* (Math|Vector|GetForwardVector _returnvalue_4) (Variables|Default|GetLineTraceRange))) "TraceTypeQuery1" false (Utilities|Array|MakeArray (Ability|GetAvatarActorfromActorInfo)) "ForDuration"))
          (bind _aspawn (Utilities|Casting|CastToPawn (.hitactor _outhit)))
          (Class|ZombieGameplayAbility|ApplyDamageEffecttoTarget _aspawn)
          (if (GameplayTags|HasMatchingGameplayTag (Variables|Default|GetOwningASC) (Variables|Default|GetCriticalTag))
            (Class|ZombieAbilitySystemComponent|RemoveGameplayTag (Variables|Default|GetOwningASC) (Variables|Default|GetCriticalTag))))))
    (:OnCompleted
      (Ability|EndAbility :!label _label))
    (:OnBlendOut
      (goto _label))
    (:OnInterrupted
      (goto _label))
    (:OnCancelled
      (goto _label))))

(event Ability|EventOnEndAbility
  (params (bWasCancelled :type Boolean)))