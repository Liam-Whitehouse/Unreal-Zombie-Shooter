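; Gameplay ability that plays the zombie spawn animation and holds the character in place until spawning finishes.
; On activation it commits, sets the ZombieCharacter's max walk speed to zero and starts the Snapper spawn montage, which keeps playing if the ability ends.
; A Gameplay.Spawn gameplay event then restores a fixed walk speed and ends the ability.
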(event Ability|EventActivateAbility
  (Ability|CommitAbility)
  (Variables|/Script/Engine.CharacterMovementComponent|SetMaxWalkSpeed (Variables|/Script/Engine.Character|GetCharacterMovement (.AsZombie%20Character (Utilities|Casting|CastToZombieCharacter (Ability|GetAvatarActorfromActorInfo)))) 0.0)
  (|PlayMontageandWaitProxy "None" "/Game/GameContent/Enemies/Zombies/MeleeZombie/Animations/AM_Snapper_Spawn.AM_Snapper_Spawn" 1.0 "None" false 1.0 0.0 false
    (:then
      (Ability|Tasks|WaitGameplayEvent "(TagName=\"Gameplay.Spawn\")" 0
        (:EventReceived
          (Variables|/Script/Engine.CharacterMovementComponent|SetMaxWalkSpeed (Variables|/Script/Engine.Character|GetCharacterMovement (.AsZombie%20Character (Utilities|Casting|CastToZombieCharacter (Ability|GetAvatarActorfromActorInfo)))) 3e+02)
          (Ability|EndAbility))))))

(event Ability|EventOnEndAbility
  (params (bWasCancelled :type Boolean)))