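; Zombie spawner actor that periodically places zombies at its SpawnLocation until the game mode's maximum count is reached.
; A two-second Delay on Tick paces an authority-only check against the game mode's cap, printing a debug message when it is full.
; Instead of creating actors, it teleports a random entry from ZombieSpawnerSystem's preloaded LoadedZombies pool, removes it from that pool and increments the game mode's count.
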(event EventBeginPlay)

(event Collision|EventActorBeginOverlap
  (params (OtherActor :type Actor%20Object%20Reference)))

(event EventTick
  (params (DeltaSeconds :type Float%20%28single-precision%29))
  (bind _returnvalue (Game|GetGameMode))
  (bind (_asbp_main_game_mode _bsuccess) (Utilities|Casting|CastToBP_MainGameMode _returnvalue))
  (Utilities|FlowControl|Delay 2.0)
  (if (Ability|HasAuthority)
    (if _bsuccess
      (bind _output_get (Variables|Default|SetGameMode _asbp_main_game_mode))
      (if (Class|MainGameMode|HasReachedMaxZombieCount _output_get)
        (Development|PrintString "Max Zombier Amount Reached")
        (else
          (bind _output_get_2 (Variables|Default|SetChosenActor (.OutItem (Utilities|Array|Random (Variables|/Script/Zombie_Shooter.ZombieSpawnerSystem|GetLoadedZombies (Subsystems|GetZombieSpawnerSystem))))))
          (Transformation|SetActorTransform _output_get_2 (Transformation|GetWorldTransform (Variables|Default|GetSpawnLocation)) false true)
          (Utilities|Array|RemoveItem (Variables|/Script/Zombie_Shooter.ZombieSpawnerSystem|GetLoadedZombies (Subsystems|GetZombieSpawnerSystem)) (Variables|Default|GetChosenActor))
          (Class|MainGameMode|AddZombieCount (Variables|Default|GetGameMode)))))))

(fn ConstructionScript)