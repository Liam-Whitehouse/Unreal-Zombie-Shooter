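; Player controller for the survivor, translating Enhanced Input actions into calls on BP_SurvivorCharacter.
; It caches player 0's pawn on BeginPlay, then forwards movement, mouse look, jump, right-click zoom and left-click hold/release.
; Movement input disables orient-rotation-to-movement while active and restores it when released.
; Escape reaches WBP_PlayerScreen through the HUD, calls ShowPauseScreen and switches the character's pause state based on the screen's visibility.
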(event Input|EnhancedActionEvents|EnhancedInputActionIA_LeftClick
  (params (ActionValue :type Boolean) (ElapsedSeconds :type Float%20%28double-precision%29) (TriggeredSeconds :type Float%20%28double-precision%29) (InputAction :type Input%20Action%20Object%20Reference :default "/Game/GameContent/Input/Actions/IA_LeftClick.IA_LeftClick"))
  (:Triggered
    (Default|LeftClickHeld (Variables|Default|GetSurvivorCharacter) (Variables|Default|GetLeftMouseInput)))
  (:Completed
    (Default|LeftClickRelease (Variables|Default|GetSurvivorCharacter))))

(event Input|EnhancedActionEvents|EnhancedInputActionIA_MoveRight
  (params (ActionValue :type Float%20%28double-precision%29) (ElapsedSeconds :type Float%20%28double-precision%29) (TriggeredSeconds :type Float%20%28double-precision%29) (InputAction :type Input%20Action%20Object%20Reference :default "/Game/GameContent/Input/Actions/IA_MoveRight.IA_MoveRight"))
  (bind _survivorcharacter (Variables|Default|GetSurvivorCharacter))
  (:Triggered
    (Default|MoveRight (Variables|Default|GetSurvivorCharacter) ActionValue))
  (:Started
    (Default|OrientRotationtoMovement _survivorcharacter false))
  (:Canceled
    (Default|OrientRotationtoMovement _survivorcharacter true :!label _label))
  (:Completed
    (goto _label)))

(event Input|EnhancedActionEvents|EnhancedInputActionIA_MouseX
  (params (ActionValue :type Float%20%28double-precision%29) (ElapsedSeconds :type Float%20%28double-precision%29) (TriggeredSeconds :type Float%20%28double-precision%29) (InputAction :type Input%20Action%20Object%20Reference :default "/Game/GameContent/Input/Actions/IA_MouseX.IA_MouseX"))
  (Default|MouseXInput (Variables|Default|GetSurvivorCharacter) ActionValue))

(event Input|EnhancedActionEvents|EnhancedInputActionIA_MouseY
  (params (ActionValue :type Float%20%28double-precision%29) (ElapsedSeconds :type Float%20%28double-precision%29) (TriggeredSeconds :type Float%20%28double-precision%29) (InputAction :type Input%20Action%20Object%20Reference :default "/Game/GameContent/Input/Actions/IA_MouseY.IA_MouseY"))
  (Default|MouseYInput (Variables|Default|GetSurvivorCharacter) ActionValue))

(event Input|EnhancedActionEvents|EnhancedInputActionIA_MoveForward
  (params (ActionValue :type Float%20%28double-precision%29) (ElapsedSeconds :type Float%20%28double-precision%29) (TriggeredSeconds :type Float%20%28double-precision%29) (InputAction :type Input%20Action%20Object%20Reference :default "/Game/GameContent/Input/Actions/IA_MoveForward.IA_MoveForward"))
  (bind _survivorcharacter (Variables|Default|GetSurvivorCharacter))
  (:Triggered
    (Default|MoveForward (Variables|Default|GetSurvivorCharacter) ActionValue))
  (:Started
    (Default|OrientRotationtoMovement _survivorcharacter false))
  (:Canceled
    (Default|OrientRotationtoMovement _survivorcharacter true :!label _label))
  (:Completed
    (goto _label)))

(event Input|EnhancedActionEvents|EnhancedInputActionIA_Jump
  (params (ActionValue :type Boolean) (ElapsedSeconds :type Float%20%28double-precision%29) (TriggeredSeconds :type Float%20%28double-precision%29) (InputAction :type Input%20Action%20Object%20Reference :default "/Game/GameContent/Input/Actions/IA_Jump.IA_Jump"))
  (:Triggered
    (Character|Jump (Variables|Default|GetSurvivorCharacter)))
  (:Canceled
    (Character|StopJumping (Variables|Default|GetSurvivorCharacter) :!label _label))
  (:Completed
    (goto _label)))

(event Input|EnhancedActionEvents|EnhancedInputActionIA_RightClick
  (params (ActionValue :type Boolean) (ElapsedSeconds :type Float%20%28double-precision%29) (TriggeredSeconds :type Float%20%28double-precision%29) (InputAction :type Input%20Action%20Object%20Reference :default "/Game/GameContent/Input/Actions/IA_RightClick.IA_RightClick"))
  (Default|CameraZoom (Variables|Default|GetSurvivorCharacter)))

(event Input|EnhancedActionEvents|EnhancedInputActionIA_Escape
  (params (ActionValue :type Boolean) (ElapsedSeconds :type Float%20%28double-precision%29) (TriggeredSeconds :type Float%20%28double-precision%29) (InputAction :type Input%20Action%20Object%20Reference :default "/Game/GameContent/Input/Actions/IA_Escape.IA_Escape"))
  (bind _aswbp_player_screen (Utilities|Casting|CastToWBP_PlayerScreen (Variables|/Script/Zombie_Shooter.PlayerHUD|GetOverlayWidget (.AsBP%20Player%20Hud (Utilities|Casting|CastToBP_PlayerHud (HUD|GetHUD))))))
  (bind _output_get (Variables|Default|SetPlayerScreen _aswbp_player_screen))
  (if (Variables|/Game/GameContent/UI/Widgets/WBP_PlayerScreen.WBP_PlayerScreen_C|GetIsPauseScreenVisible _output_get)
    (Default|ShowPauseScreen (Variables|Default|GetPlayerScreen))
    (Default|UnPauseState (Variables|Default|GetSurvivorCharacter))
    (else
      (Default|ShowPauseScreen (Variables|Default|GetPlayerScreen))
      (Default|PauseState (Variables|Default|GetSurvivorCharacter)))))

(event EventBeginPlay
  (bind _asbp_survivor_character (Utilities|Casting|CastToBP_SurvivorCharacter (Game|Player|GetPlayerPawn 0)))
  (Variables|Default|SetSurvivorCharacter _asbp_survivor_character))

(event EventTick
  (params (DeltaSeconds :type Float%20%28single-precision%29)))

(fn ConstructionScript)