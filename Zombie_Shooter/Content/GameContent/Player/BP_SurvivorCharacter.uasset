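; Player survivor character Blueprint that handles look, movement and click-to-ability input through the Gameplay Ability System.
; Look and move events are ignored while Dead or Paused tags are present; horizontal look yaws both controller and actor.
; Held left click passes its input tag to ZombieAbilitySystemComponent, blocked only by Dead.
; Pause events toggle the Paused tag, and another event sets orient-rotation-to-movement; click release and zoom are empty.
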(event Custom|MouseXInput
  (params (ActionValue :type Float%20%28double-precision%29))
  (if (not (or (GameplayTags|HasMatchingGameplayTag (Ability|GetAbilitySystemComponent 0) "(TagName=\"Gameplay.Dead\")") (GameplayTags|HasMatchingGameplayTag (Ability|GetAbilitySystemComponent 0) "(TagName=\"Gameplay.Paused\")")))
    (Pawn|Input|AddControllerYawInput ActionValue)
    (Class|Actor|AddActorWorldRotation (Math|Rotator|MakeRotator 0.0 0.0 ActionValue))))

(event Custom|MouseYInput
  (params (ActionValue :type Float%20%28double-precision%29))
  (if (not (or (GameplayTags|HasMatchingGameplayTag (Ability|GetAbilitySystemComponent 0) "(TagName=\"Gameplay.Dead\")") (GameplayTags|HasMatchingGameplayTag (Ability|GetAbilitySystemComponent 0) "(TagName=\"Gameplay.Paused\")")))
    (Pawn|Input|AddControllerPitchInput (* ActionValue -1.0))))

(event Custom|LeftClickHeld
  (params (InputTag :type Gameplay%20Tag%20Structure))
  (if (not (GameplayTags|HasMatchingGameplayTag (Ability|GetAbilitySystemComponent 0) "(TagName=\"Gameplay.Dead\")"))
    (bind _aszombie_ability_system_component (Utilities|Casting|CastToZombieAbilitySystemComponent (Ability|GetAbilitySystemComponent 0)))
    (Class|ZombieAbilitySystemComponent|AbilityInputTagPressed _aszombie_ability_system_component InputTag)))

(event Custom|LeftClickRelease)

(event Custom|MoveForward
  (params (ActionValue :type Float%20%28double-precision%29))
  (if (not (or (GameplayTags|HasMatchingGameplayTag (Ability|GetAbilitySystemComponent 0) "(TagName=\"Gameplay.Dead\")") (GameplayTags|HasMatchingGameplayTag (Ability|GetAbilitySystemComponent 0) "(TagName=\"Gameplay.Paused\")")))
    (Class|SurvivorCharacter|MovePlayerForward ActionValue)))

(event Custom|OrientRotationToMovement
  (params (bShouldRotateToMovement :type Boolean))
  (Variables|/Script/Engine.CharacterMovementComponent|SetbOrientRotationToMovement (Variables|Character|GetCharacterMovement) bShouldRotateToMovement))

(event Custom|MoveRight
  (params (ActionValue :type Float%20%28double-precision%29))
  (if (not (or (GameplayTags|HasMatchingGameplayTag (Ability|GetAbilitySystemComponent 0) "(TagName=\"Gameplay.Dead\")") (GameplayTags|HasMatchingGameplayTag (Ability|GetAbilitySystemComponent 0) "(TagName=\"Gameplay.Paused\")")))
    (Class|SurvivorCharacter|MovePlayerRight ActionValue)))

(event Custom|CameraZoom)

(event Custom|PauseState
  (Class|ZombieAbilitySystemComponent|AddGameplayTag (.AsZombie%20Ability%20System%20Component (Utilities|Casting|CastToZombieAbilitySystemComponent (Ability|GetAbilitySystemComponent 0))) (GameplayTags|MakeLiteralGameplayTag "(TagName=\"Gameplay.Paused\")")))

(event Custom|UnPauseState
  (Class|ZombieAbilitySystemComponent|RemoveGameplayTag (.AsZombie%20Ability%20System%20Component (Utilities|Casting|CastToZombieAbilitySystemComponent (Ability|GetAbilitySystemComponent 0))) (GameplayTags|MakeLiteralGameplayTag "(TagName=\"Gameplay.Paused\")")))

(event EventBeginPlay)

(event Collision|EventActorBeginOverlap
  (params (OtherActor :type Actor%20Object%20Reference)))

(event EventTick
  (params (DeltaSeconds :type Float%20%28single-precision%29)))

(fn ConstructionScript)